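; Ability system function library whose ApplyHitDamageTarget handles hit reaction and damage after an attack lands.
; With valid hit data, target and ASC, it always sends the target an attack-detection event.
; Unless the target is Invincible, it sends a BeHit event carrying the extra data and hit context, then applies GE_Damage with SetByCaller base damage.
; The target's own ASC creates the damage spec and context, so the attacker's context isn't carried into it.
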(fn `ApplyHitDamageTarget`
  (params (InBeHitActor :type "WKCharacterBase Object Reference") (InHitEventData :type "GameplayEventData Structure") (InBaseDamage :type "Float (double-precision)") (BeHitExtraData :type "WKCharacterBeHitEventExtraData Object Reference"))
  (locals (InstigatorASC :type "WKAbilitySystemComponent Object Reference") (BeHitASC :type "WKAbilitySystemComponent Object Reference"))
  (bind _behitasc (`local.BeHitASC`))
  (`/Engine/EditorBlueprintResources/StandardMacros.IsValid` BeHitExtraData
    (:`Is Valid`
      (`/Engine/EditorBlueprintResources/StandardMacros.IsValid` InBeHitActor
        (:`Is Valid`
          (set `local.BeHitASC` (`WKGameplayStatics.GetWKAbilitySystemComponent` InBeHitActor))
          (`/Engine/EditorBlueprintResources/StandardMacros.IsValid` (`local.BeHitASC`)
            (:`Is Valid`
              ;[1 1 1] 处理攻击命中后的Hit反应、伤害
              (`AbilitySystemBlueprintLibrary.SendGameplayEventToActor` (`local.InBeHitActor`) (struct :`TagName` "Gameplay.Message.Attack.Detection"))
              (if (not (`WKAbilitySystemComponent.HasMatchingGameplayTagExactly` (`local.BeHitASC`) (struct :`TagName` "Gameplay.State.Invincible")))
                (`AbilitySystemBlueprintLibrary.SendGameplayEventToActor` (`local.InBeHitActor`) (struct :`TagName` "Gameplay.Event.BeHit") (make `GameplayEventData` (struct) null null (`local.BeHitExtraData`) null (`.ContextHandle` (break `GameplayEventData` (`local.InHitEventData`)))))
                (bind _returnvalue (`AbilitySystemBlueprintLibrary.AssignTagSetByCallerMagnitude` (`AbilitySystemComponent.MakeOutgoingSpec` _behitasc "/Game/_Game/AbilitySystem/GameplayEffect/GE_Damage.GE_Damage_C" 1.0 (`AbilitySystemComponent.MakeEffectContext` _behitasc)) (struct :`TagName` "SetByCaller.Amount.BaseDamage") (`local.InBaseDamage`)))
                (`AbilitySystemComponent.BP_ApplyGameplayEffectSpecToSelf` (`local.BeHitASC`) _returnvalue)))))))))