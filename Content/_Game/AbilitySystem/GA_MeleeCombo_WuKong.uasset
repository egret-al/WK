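; Gameplay Ability for WuKong's melee combo, playing one step of the attack chain per activation.
; GetComboMontage uses the character's current combo index to pick a section of AM_MeleeCombo_WuKong, and the fifth section also makes the character jump.
; Damage hit events received during the montage make the target play its hit montage relative to WuKong.
; The ability ends when the montage finishes, blends out or is stopped.
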(event `self.K2_ActivateAbility`
  (bind (_montage _name) (`self.GetComboMontage`))
  (set `self.Montage` _montage)
  (set `self.SectionName` _name)
  (`|ExecutionSequence`
    (:`then_0`
      (if (== (`self.SectionName`) (`|GetArrayItem` (`self.ComboNames`) 4))
        (`Character.Jump` (`self.GetWKCharacterFromActorInfo`))))
    (:`then_1`
      (bind (_asynctaskproxy _eventtag _eventdata) (`WKAbilityTask_PlayMontageAndWaitForEvent.PlayMontageAndWaitForEvent` "Combo" (`self.Montage`) (struct :`GameplayTags` (struct :`(TagName` "Gameplay.Message.Damage.Hit"))) 1.0 (`self.SectionName`))
        (:`OnCompleted`
          (`self.K2_EndAbility` :!label _label))
        (:`OnBlendOut`
          (goto _label))
        (:`OnInterrupted`
          (goto _label))
        (:`OnCancelled`
          (goto _label))
        (:`OnMontageStop`
          (goto _label))
        (:`EventReceived`
          (if (== _eventtag (struct :`TagName` "Gameplay.Message.Damage.Hit"))
            (bind _aswkcharacter_base (cast `WKCharacterBase` (`.Target` (break `GameplayEventData` _eventdata))))
            (`WKCharacterBase.PlayHitMontage` _aswkcharacter_base (`self.GetWKCharacterFromActorInfo`))))))))

(event `self.K2_OnEndAbility`
  (params (bWasCancelled :type Boolean)))

(fn `GetComboMontage`
  (returns (Montage :type "AnimMontage Object Reference") (Name :type Name))
  (return "/Game/_Game/Character/WuKong/Animation/AnimMontage/AM_MeleeCombo_WuKong.AM_MeleeCombo_WuKong" (`|GetArrayItem` (`self.ComboNames`) (`WKCharacterBase.CurrentMeleeComboIndex` (`self.GetWKCharacterFromActorInfo`)))))