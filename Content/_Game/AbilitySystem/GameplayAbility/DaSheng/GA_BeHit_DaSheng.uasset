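; Hit-reaction ability for DaSheng, activatable only while the character's resilience is below a fixed threshold.
; It picks a montage and section from the hit event's instigator, hit result and impact, then plays it, ending when the montage does.
; A ShouldMove event unblocks movement so move input can cancel the reaction, and a BeHitEnd event ends it after a random delay capped by event magnitude.
; The knockback impulse logic is disconnected.
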(event `self.K2_ActivateAbilityFromEvent`
  (params (EventData :type "GameplayEventData Structure (by ref)"))
  (bind _output_get (set `self.BeHitEventData` EventData))
  (bind _aswkcharacter_be_hit_event_extra_data (cast `WKCharacterBeHitEventExtraData` (`.OptionalObject` (break `GameplayEventData` _output_get)))
    (:`then`
      (bind _output_get_2 (set `self.BeHitEventExtraData` _aswkcharacter_be_hit_event_extra_data))
      (bind (_outhitmontage _outsectionname _returnvalue) (`WKGameplayStatics.CalculateBeHitInfo` (`WKCharacterBeHitEventExtraData.Instigator` _aswkcharacter_be_hit_event_extra_data) (`self.GetWKCharacterFromActorInfo`) (`AbilitySystemBlueprintLibrary.EffectContextGetHitResult` (`.ContextHandle` (break `GameplayEventData` (`self.BeHitEventData`)))) (`WKCharacterBeHitEventExtraData.BeHitImpact` _output_get_2)))
      (set `self.BeHitMontage` _outhitmontage)
      (set `self.SectionName` _outsectionname)
      (if _returnvalue
        (bind (_asynctaskproxy _eventtag _eventdata) (`WKAbilityTask_PlayMontageAndWaitForEvent.PlayMontageAndWaitForEvent` "None" (`self.BeHitMontage`) (struct :`GameplayTags` (struct :`(TagName` "Gameplay.Message.Damage.BeHitEnd"))) 1.0 (`self.SectionName`))
          (:`then`
            (`AbilityTask_WaitGameplayEvent.WaitGameplayEvent` (struct :`TagName` "Gameplay.Message.ShouldMove") null
              (:`then`
                (`WKAbilityTask_WaitMoveInput.WaitMoveInput` false
                  (:`then`)
                  (:`OnMoveInput`
                    (if (`self.CanMove`)
                      (`self.K2_EndAbility`)))))
              (:`EventReceived`
                (set `self.CanMove` true)
                (`self.RemoveGameplayTag` (struct :`TagName` "Gameplay.State.Input.BlockMove")))))
          (:`OnCompleted`
            (`self.K2_EndAbility` :!label _label))
          (:`OnBlendOut`
            (goto _label))
          (:`OnInterrupted`
            (goto _label))
          (:`OnCancelled`
            (goto _label))
          (:`OnMontageStop`
            (goto _label))
          (:`EventReceived`
            ;[1 1 1] 可以提前结束，随机一个时间，tick到后结束
            (if (== _eventtag (struct :`TagName` "Gameplay.Message.Damage.BeHitEnd"))
              (bind _output_get_3 (set `self.DelayEnd` (`KismetMathLibrary.RandomFloatInRange` 0.0 (`.EventMagnitude` (break `GameplayEventData` _eventdata)))))
              (if (== _output_get_3 0.0)
                (`self.K2_EndAbility`)
                (else
                  (set `self.CurTime` 0.0)
                  (bind (_asynctaskproxy_2 _deltatime) (`WKAbilityTask_TickTask.TickTask` -1.0)
                    (:`OnTickDelegate`
                      (bind _output_get_4 (set `self.CurTime` (+ _deltatime (`self.CurTime`))))
                      (if (> _output_get_4 (`self.DelayEnd`))
                        (`self.K2_EndAbility`)))))))))
        (else
          (`KismetSystemLibrary.PrintString` "大圣的受击配置没有找到合适的动画，请检查配置文件" true true (struct :`R` 1.0 :`G` 0.033493 :`A` 1.0))
          (`self.K2_EndAbility`))))
    (:`CastFailed`
      (`self.K2_EndAbility`))))

(event `self.K2_OnEndAbility`
  (params (bWasCancelled :type Boolean))
  (set `self.CanMove` false))

(fn `K2_CanActivateAbility`
  (params (ActorInfo :type "GameplayAbilityActorInfo Structure") (Handle :type "GameplayAbilitySpecHandle Structure"))
  (returns (RelevantTags :type "GameplayTagContainer Structure") (ReturnValue :type Boolean))
  ;[1 1 1] 韧性值检查
  (return (struct) (< (`WKHealthComponent.GetResilience` (`WKCharacterBase.HealthComponent` (`self.GetWKCharacterFromActorInfo`))) 50.0)))