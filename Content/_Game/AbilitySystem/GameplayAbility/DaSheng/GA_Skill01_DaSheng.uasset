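; GA_Skill01_DaSheng is DaSheng's first skill ability, a montage-driven attack that damages characters it hits.
; On activation it commits, plays AM_Skill01_DaSheng and waits for Gameplay.Message.Damage.Hit events.
; Each hit casts the target to WKCharacterBase and, if its ability system component is valid, applies damage and impact using the ability's data asset.
; The ability ends when the montage completes, blends out, stops or is interrupted or cancelled.
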(event `self.K2_ActivateAbility`
  (`self.K2_CommitAbility`)
  (bind (_asynctaskproxy _eventtag _eventdata) (`WKAbilityTask_PlayMontageAndWaitForEvent.PlayMontageAndWaitForEvent` "None" "/Game/_Game/Character/DaSheng/Animation/AnimMontage/AM_Skill01_DaSheng.AM_Skill01_DaSheng" (struct :`GameplayTags` (struct :`(TagName` "Gameplay.Message.Damage.Hit"))))
    (:`OnCompleted`
      (`self.K2_EndAbility` :!label _label))
    (:`OnBlendOut`
      (goto _label))
    (:`OnInterrupted`
      (goto _label))
    (:`OnCancelled`
      (goto _label))
    (:`OnMontageStop`
      (goto _label))
    (:`EventReceived`
      (if (== _eventtag (struct :`TagName` "Gameplay.Message.Damage.Hit"))
        (bind _output_get (set `self.HitEventData` _eventdata))
        (bind _aswkcharacter_base (cast `WKCharacterBase` (`.Target` (break `GameplayEventData` _output_get))))
        (bind _output_get_2 (set `self.HitActor` _aswkcharacter_base))
        (bind _output_get_3 (set `self.HitActorASC` (`WKGameplayStatics.GetWKAbilitySystemComponent` _output_get_2)))
        (`/Engine/EditorBlueprintResources/StandardMacros.IsValid` _output_get_3
          (:`Is Valid`
            (`/Game/_Game/AbilitySystem/BP_AbilityFunctionLibrary.ApplyHitDamageTarget` (`self.GetWKCharacterFromActorInfo`) (`self.HitActor`) (`self.AbilityDataAsset`) (`self.HitEventData`) 30.0 (`self.HitImpact`))))))))

(event `self.K2_OnEndAbility`
  (params (bWasCancelled :type Boolean)))