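; Gameplay ability for DaSheng's Skill 15, a montage-driven attack that runs only while the character has a valid attack lock target.
; It commits, checks the target (ending at once without one), then plays the skill montage and listens for damage hit gameplay events.
; Each hit on a character with an ability system component builds be-hit extra data and applies base damage.
; The ability ends when the montage finishes, blends out or is stopped.
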(event `self.K2_ActivateAbility`
  (`self.K2_CommitAbility`)
  (set `self.CurrentTarget` (`WKCharacterBase.GetCurrentAttackLockTarget` (`self.GetWKCharacterFromActorInfo`)))
  (`self.CurrentTarget`
    (:`then`
      (bind (_asynctaskproxy _eventtag _eventdata) (`WKAbilityTask_PlayMontageAndWaitForEvent.PlayMontageAndWaitForEvent` "None" "/Game/_Game/Character/DaSheng/Animation/AnimMontage/AM_Skill15_DaSheng.AM_Skill15_DaSheng" (struct :`GameplayTags` (struct :`(TagName` "Gameplay.Message.Damage.Hit"))))
        (:`OnCompleted`
          (`self.K2_EndAbility` :!label _label))
        (:`OnBlendOut`
          (goto _label))
        (:`OnInterrupted`
          (goto _label))
        (:`OnCancelled`
          (goto _label))
        (:`OnMontageStop`
          (goto _label))
        (:`EventReceived`
          (if (== _eventtag (struct :`TagName` "Gameplay.Message.Damage.Hit"))
            (bind _output_get (set `self.HitEventData` _eventdata))
            (bind _aswkcharacter_base (cast `WKCharacterBase` (`.Target` (break `GameplayEventData` _output_get))))
            (bind _output_get_2 (set `self.HitActor` _aswkcharacter_base))
            (bind _output_get_3 (set `self.HitActorASC` (`WKGameplayStatics.GetWKAbilitySystemComponent` _output_get_2)))
            (`/Engine/EditorBlueprintResources/StandardMacros.IsValid` _output_get_3
              (:`Is Valid`
                (bind _returnvalue (`|GenericCreateObject` "/Script/BlackWK.WKCharacterBeHitEventExtraData"))
                (set `WKCharacterBeHitEventExtraData.Instigator` (`self.GetWKCharacterFromActorInfo`) _returnvalue)
                (set `WKCharacterBeHitEventExtraData.AbilityDataAsset` (`self.AbilityDataAsset`) _returnvalue)
                (set `WKCharacterBeHitEventExtraData.BeHitImpact` (`self.HitImpact`) _returnvalue)
                (`/Game/_Game/AbilitySystem/BP_AbilityFunctionLibrary.ApplyHitDamageTarget` (`self.HitActor`) (`self.HitEventData`) 10.0 _returnvalue)))))))
    (:`else`
      (`self.K2_EndAbility`))))

(event `self.K2_OnEndAbility`
  (params (bWasCancelled :type Boolean)))