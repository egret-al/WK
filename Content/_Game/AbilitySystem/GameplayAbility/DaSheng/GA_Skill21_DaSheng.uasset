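; Gameplay ability for DaSheng's Skill 21, an immobilize spell that roots the currently locked attack target.
; It commits first, then ends immediately if no valid lock target exists, otherwise plays the skill montage.
; A root message event from the montage task re-reads the lock target and sends it a Rooted gameplay event.
; Any montage completion, blend-out, interruption, cancel or stop ends the ability.
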(event `self.K2_ActivateAbility`
  (`self.K2_CommitAbility`)
  (set `self.CurrentTarget` (`WKCharacterBase.GetCurrentAttackLockTarget` (`self.GetWKCharacterFromActorInfo`)))
  (`self.CurrentTarget`
    (:`then`
      (bind (_asynctaskproxy _eventtag) (`WKAbilityTask_PlayMontageAndWaitForEvent.PlayMontageAndWaitForEvent` "None" "/Game/_Game/Character/DaSheng/Animation/AnimMontage/AM_Skill21_DaSheng.AM_Skill21_DaSheng" (struct :`GameplayTags` (struct :`(TagName` "Gameplay.Message.Root"))))
        (:`OnCompleted`
          (`self.K2_EndAbility` :!label _label))
        (:`OnBlendOut`
          (goto _label))
        (:`OnInterrupted`
          (goto _label))
        (:`OnCancelled`
          (goto _label))
        (:`OnMontageStop`
          (goto _label))
        (:`EventReceived`
          (if (== _eventtag (struct :`TagName` "Gameplay.Message.Root"))
            (`KismetSystemLibrary.PrintString` "释放定身")
            (`AbilitySystemBlueprintLibrary.SendGameplayEventToActor` (`WKCharacterBase.GetCurrentAttackLockTarget` (`self.GetWKCharacterFromActorInfo`)) (struct :`TagName` "Gameplay.Event.Rooted"))))))
    (:`else`
      (`self.K2_EndAbility`))))

(event `self.K2_OnEndAbility`
  (params (bWasCancelled :type Boolean)))