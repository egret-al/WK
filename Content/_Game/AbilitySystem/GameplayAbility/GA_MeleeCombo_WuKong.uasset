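; Gameplay ability for WuKong's melee combo, playing the montage section selected by the character's current combo index.
; The section at name index 4 also triggers a jump.
; Hit events play the target's hit reaction and apply GE_Damage through the target's own ability system, unless it is invincible.
; A ShouldMove event lifts the movement block, letting move input end the ability and clear the combo index; montage completion or interruption also ends it.
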(event `self.K2_ActivateAbility`
  (bind (_montage _name) (`self.GetComboMontage`))
  (bind _returnvalue (`self.GetWKCharacterFromActorInfo`))
  (set `self.Montage` _montage)
  (set `self.SectionName` _name)
  (`|ExecutionSequence`
    (:`then_0`
      (if (== (`self.SectionName`) (`|GetArrayItem` (`self.ComboNames`) 4))
        (`Character.Jump` (`self.GetWKCharacterFromActorInfo`))))
    (:`then_1`
      (bind (_asynctaskproxy _eventtag _eventdata) (`WKAbilityTask_PlayMontageAndWaitForEvent.PlayMontageAndWaitForEvent` "Combo" (`self.Montage`) (struct :`GameplayTags` (struct :`(TagName` "Gameplay.Message.Damage.Hit"))) 1.0 (`self.SectionName`))
        (:`then`
          (`AbilityTask_WaitGameplayEvent.WaitGameplayEvent` (struct :`TagName` "Gameplay.Message.ShouldMove") null
            (:`then`
              (`WKAbilityTask_WaitMoveInput.WaitMoveInput` false
                (:`OnMoveInput`
                  (if (`self.CanMove`)
                    (`/Engine/EditorBlueprintResources/StandardMacros.IsValid` _returnvalue
                      (:`Is Valid`
                        (`WKCharacterBase.ClearMeleeComboIndex` _returnvalue)
                        (`self.K2_EndAbility`)))))))
            (:`EventReceived`
              (set `self.CanMove` true)
              (`self.RemoveGameplayTag` (struct :`TagName` "Gameplay.State.Input.BlockMove")))))
        (:`OnCompleted`
          (`self.K2_EndAbility` :!label _label))
        (:`OnBlendOut`
          (goto _label))
        (:`OnInterrupted`
          (goto _label))
        (:`OnCancelled`
          (goto _label))
        (:`OnMontageStop`
          (goto _label))
        (:`EventReceived`
          (if (== _eventtag (struct :`TagName` "Gameplay.Message.Damage.Hit"))
            ;[1 1 1] 命中到目标了
            (bind _aswkcharacter_base (cast `WKCharacterBase` (`.Target` (break `GameplayEventData` _eventdata))))
            (if (not (`WKAbilitySystemComponent.HasMatchingGameplayTagExactly` (`WKGameplayStatics.GetWKAbilitySystemComponent` _aswkcharacter_base) (struct :`TagName` "Gameplay.State.Invincible")))
              (`WKCharacterBase.PlayHitMontage` _aswkcharacter_base (`self.GetWKCharacterFromActorInfo`))
              (bind _returnvalue_2 (`WKGameplayStatics.GetWKAbilitySystemComponent` _aswkcharacter_base))
              (`AbilitySystemComponent.BP_ApplyGameplayEffectSpecToSelf` _returnvalue_2 (`AbilitySystemComponent.MakeOutgoingSpec` _returnvalue_2 "/Game/_Game/AbilitySystem/GameplayEffect/GE_Damage.GE_Damage_C" 1.0 (`AbilitySystemComponent.MakeEffectContext` _returnvalue_2))))))))))

(event `self.K2_OnEndAbility`
  (params (bWasCancelled :type Boolean))
  (`parent.K2_OnEndAbility` bWasCancelled)
  (set `self.CanMove` false))

(fn `GetComboMontage`
  (returns (Montage :type "AnimMontage Object Reference") (Name :type Name))
  (return "/Game/_Game/Character/WuKong/Animation/AnimMontage/AM_MeleeCombo_WuKong.AM_MeleeCombo_WuKong" (`|GetArrayItem` (`self.ComboNames`) (`WKCharacterBase.CurrentMeleeComboIndex` (`self.GetWKCharacterFromActorInfo`)))))