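; DaSheng's Skill01 gameplay ability, which plays the skill's attack montage and listens for damage hit events.
; A montage task runs on activation and ends the ability when it completes, blends out, stops, is interrupted or is cancelled.
; On a hit event targeting a WK character, it checks for the Invincible state tag and, if absent, only prints the target's name, with no damage applied here.
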(event `self.K2_ActivateAbility`
  (bind (_asynctaskproxy _eventtag _eventdata) (`WKAbilityTask_PlayMontageAndWaitForEvent.PlayMontageAndWaitForEvent` "None" "/Game/_Game/Character/DaSheng/Animation/AnimMontage/AM_Skill01_DaSheng.AM_Skill01_DaSheng" (struct :`GameplayTags` (struct :`(TagName` "Gameplay.Message.Damage.Hit"))))
    (:`OnCompleted`
      (`self.K2_EndAbility` :!label _label))
    (:`OnBlendOut`
      (goto _label))
    (:`OnInterrupted`
      (goto _label))
    (:`OnCancelled`
      (goto _label))
    (:`OnMontageStop`
      (goto _label))
    (:`EventReceived`
      (if (== _eventtag (struct :`TagName` "Gameplay.Message.Damage.Hit"))
        (bind (_eventtag_2 _instigator _target) (break `GameplayEventData` _eventdata))
        (cast `WKCharacterBase` _target)
        (if (not (`WKAbilitySystemComponent.HasMatchingGameplayTagExactly` (`WKGameplayStatics.GetWKAbilitySystemComponent` null) (struct :`TagName` "Gameplay.State.Invincible")))
          (`KismetSystemLibrary.PrintString` (`KismetSystemLibrary.GetDisplayName` _target)))))))