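; Gameplay ability that plays Wukong's hit reaction when triggered by a gameplay event.
; It derives montage and section from instigator, hit result and impact magnitude, then resets the melee combo index and enables root motion.
; A ShouldMove event removes the move-input block, letting movement input end the reaction early.
; Montage exits also end the ability, which disables root motion again on end.
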(event `self.K2_ActivateAbilityFromEvent`
  (params (EventData :type "GameplayEventData Structure (by ref)"))
  (bind _returnvalue (`self.GetWKCharacterFromActorInfo`))
  (bind _returnvalue_2 (`WKCharacterBase.GetWKSkeletalMeshComponent` _returnvalue))
  (bind _output_get (set `self.BeHitEventData` EventData))
  (bind (_eventtag _instigator _target _optionalobject _optionalobject2 _contexthandle _instigatortags _targettags _eventmagnitude) (break `GameplayEventData` _output_get))
  (bind _aswkcharacter_base (cast `WKCharacterBase` _instigator)
    (:`then`
      (bind (_outhitmontage _outsectionname _returnvalue_3) (`WKGameplayStatics.CalculateBeHitInfo` _aswkcharacter_base (`self.GetWKCharacterFromActorInfo`) (`AbilitySystemBlueprintLibrary.EffectContextGetHitResult` _contexthandle) _eventmagnitude))
      (set `self.BeHitMontage` _outhitmontage)
      (set `self.SectionName` _outsectionname)
      (if _returnvalue_3
        (`|ExecutionSequence`
          (:`then_0`
            (`/Engine/EditorBlueprintResources/StandardMacros.IsValid` _returnvalue
              (:`Is Valid`
                (`WKCharacterBase.ClearMeleeComboIndex` _returnvalue)
                (`/Engine/EditorBlueprintResources/StandardMacros.IsValid` _returnvalue_2
                  (:`Is Valid`
                    (`WKSkeletalMeshComponent.SetDisableRootMotion` _returnvalue_2 false))))))
          (:`then_1`
            (`WKAbilityTask_PlayMontageAndWaitForEvent.PlayMontageAndWaitForEvent` "None" (`self.BeHitMontage`) (struct) 1.0 (`self.SectionName`)
              (:`then`
                (`AbilityTask_WaitGameplayEvent.WaitGameplayEvent` (struct :`TagName` "Gameplay.Message.ShouldMove") null
                  (:`then`
                    (`WKAbilityTask_WaitMoveInput.WaitMoveInput` false
                      (:`OnMoveInput`
                        (if (`self.CanMove`)
                          (`self.K2_EndAbility`)))))
                  (:`EventReceived`
                    (set `self.CanMove` true)
                    (`self.RemoveGameplayTag` (struct :`TagName` "Gameplay.State.Input.BlockMove")))))
              (:`OnCompleted`
                (`self.K2_EndAbility` :!label _label))
              (:`OnBlendOut`
                (goto _label))
              (:`OnInterrupted`
                (goto _label))
              (:`OnCancelled`
                (goto _label))
              (:`OnMontageStop`
                (goto _label)))))
        (else
          (`self.K2_EndAbility`))))
    (:`CastFailed`
      (`self.K2_EndAbility`))))

(event `self.K2_OnEndAbility`
  (params (bWasCancelled :type Boolean))
  (bind _returnvalue (`self.GetWKCharacterFromActorInfo`))
  (bind _returnvalue_2 (`WKCharacterBase.GetWKSkeletalMeshComponent` _returnvalue))
  (set `self.CanMove` false)
  (`/Engine/EditorBlueprintResources/StandardMacros.IsValid` _returnvalue
    (:`Is Valid`
      (`/Engine/EditorBlueprintResources/StandardMacros.IsValid` _returnvalue_2
        (:`Is Valid`
          (`WKSkeletalMeshComponent.SetDisableRootMotion` _returnvalue_2 true))))))