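; Wukong's charged attack ability, which builds stick energy while the input is held and spends all of it on release.
; A charge montage plays while a GameplayEffect accumulates energy; input release or full energy triggers the attack once.
; Current energy selects one of four tiers, setting montage section, damage and impact.
; The attack runs in Flying movement, applies damage on montage hit events, and restores Walking when the ability ends.
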(event `self.K2_ActivateAbility`
  (set `self.HasRelease` false)
  (bind _asynctaskproxy (`WKAbilityTask_PlayMontageAndWaitForEvent.PlayMontageAndWaitForEvent` "None" "/Game/_Game/Character/WuKong/Animation/AnimMontage/AM_Charge.AM_Charge")
    (:`then`
      (set `self.AbilityTask_ChargeLoop` _asynctaskproxy)
      (set `self.OwnerASC` (`self.GetWKAbilitySystemComponentFromActorInfo`))
      ;[1 1 1] 主动释放蓄力技
      (`WKAbilityTask_WaitInputRelease.WKWaitReleaseWithInput` "Charge"
        (:`then`
          ;[1 1 1] 持续积攒棍势
          (bind _ownerasc (`self.OwnerASC`)
            (:`then`
              (bind _returnvalue (`AbilitySystemBlueprintLibrary.AssignTagSetByCallerMagnitude` (`AbilitySystemComponent.MakeOutgoingSpec` _ownerasc "/Game/_Game/AbilitySystem/GameplayEffect/WuKong/GE_ChargeStickEnergy.GE_ChargeStickEnergy_C" 0.0 (`AbilitySystemComponent.MakeEffectContext` _ownerasc)) (struct :`TagName` "SetByCaller.Amount.StickEnergy") 3.0))
              (bind _returnvalue_2 (`AbilitySystemComponent.BP_ApplyGameplayEffectSpecToSelf` (`self.OwnerASC`) _returnvalue))
              (set `self.ChargeStickEnergyEffectHandle` _returnvalue_2)
              ;[1 1 1] 如果棍势积攒到了最大，直接释放
              (`WKAbilityTask_WaitStickEnergyHasMax.WaitStickEnergyHasMax`
                (:`OnMaxDelegate`
                  (`self.ReleaseChargeAttack`))))
            (:`else`)))
        (:`OnRelease`
          (`self.ReleaseChargeAttack`))))))

(event `self.K2_OnEndAbility`
  (params (bWasCancelled :type Boolean))
  (`CharacterMovementComponent.SetMovementMode` (`Character.CharacterMovement` (`self.GetWKCharacterFromActorInfo`)) "MOVE_Walking" 0)
  (bind _ownerasc (`self.OwnerASC`)
    (:`then`
      (`AbilitySystemComponent.RemoveActiveGameplayEffect` _ownerasc (`self.ChargeStickEnergyEffectHandle`) -1))
    (:`else`)))

(event `ReleaseChargeAttack`
  (bind (_secctionname _coststickenergy _basedamage _hitimpact) (`self.GetChargeAttackInfoByStickEnergy`))
  (if (not (`self.HasRelease`))
    (set `self.HasRelease` true)
    (`|ExecutionSequence`
      (:`then_0`
        ;[1 1 1] 取消持续恢复棍势的GE
        (bind _ownerasc (`self.OwnerASC`)
          (:`then`
            (`AbilitySystemComponent.RemoveActiveGameplayEffect` _ownerasc (`self.ChargeStickEnergyEffectHandle`) -1)
            (`/Engine/EditorBlueprintResources/StandardMacros.IsValid` (`self.AbilityTask_ChargeLoop`)
              (:`Is Valid`
                (`GameplayTask.EndTask` (`self.AbilityTask_ChargeLoop`)))))
          (:`else`)))
      (:`then_1`
        ;[1 1 1] 释放蓄力攻击并且扣除棍势
        (set `self.SectionName` _secctionname)
        (set `self.CostStickEnergy` _coststickenergy)
        (set `self.ChargeBaseDamage` _basedamage)
        (set `self.ChargeHitImpact` _hitimpact)
        (bind (_asynctaskproxy _eventtag _eventdata) (`WKAbilityTask_PlayMontageAndWaitForEvent.PlayMontageAndWaitForEvent` "None" "/Game/_Game/Character/WuKong/Animation/AnimMontage/AM_ChargeAttack.AM_ChargeAttack" (struct :`GameplayTags` (struct :`(TagName` "Gameplay.Message.Damage.Hit"))) 1.0 (`self.SectionName`))
          (:`then`
            (`CharacterMovementComponent.SetMovementMode` (`Character.CharacterMovement` (`self.GetWKCharacterFromActorInfo`)) "MOVE_Flying" 0)
            (bind _ownerasc_2 (`self.OwnerASC`)
              (:`then`
                (bind _returnvalue (`AbilitySystemBlueprintLibrary.AssignTagSetByCallerMagnitude` (`AbilitySystemComponent.MakeOutgoingSpec` _ownerasc_2 "/Game/_Game/AbilitySystem/GameplayEffect/WuKong/GE_StickEnergy.GE_StickEnergy_C" 1.0 (`AbilitySystemComponent.MakeEffectContext` _ownerasc_2)) (struct :`TagName` "SetByCaller.Amount.StickEnergy") (* (`self.CostStickEnergy`) -1.0)))
                (`AbilitySystemComponent.BP_ApplyGameplayEffectSpecToSelf` (`self.OwnerASC`) _returnvalue))
              (:`else`)))
          (:`OnBlendOut`
            (`self.K2_EndAbility` :!label _label))
          (:`OnInterrupted`
            (goto _label))
          (:`OnCancelled`
            (goto _label))
          (:`OnMontageStop`
            (goto _label))
          (:`EventReceived`
            ;[1 1 1] 命中目标，进行伤害判定
            (if (== _eventtag (struct :`TagName` "Gameplay.Message.Damage.Hit"))
              (bind _output_get (set `self.HitEventData` _eventdata))
              (bind _aswkcharacter_base (cast `WKCharacterBase` (`.Target` (break `GameplayEventData` _output_get))))
              (set `self.HitActor` _aswkcharacter_base)
              (bind _output_get_2 (set `self.HitActorASC` (`WKGameplayStatics.GetWKAbilitySystemComponent` _aswkcharacter_base)))
              (`/Engine/EditorBlueprintResources/StandardMacros.IsValid` _output_get_2
                (:`Is Valid`
                  (bind _returnvalue_2 (`|GenericCreateObject` "/Script/BlackWK.WKCharacterBeHitEventExtraData"))
                  (set `WKCharacterBeHitEventExtraData.Instigator` (`self.GetWKCharacterFromActorInfo`) _returnvalue_2)
                  (set `WKCharacterBeHitEventExtraData.AbilityDataAsset` (`self.AbilityDataAsset`) _returnvalue_2)
                  (set `WKCharacterBeHitEventExtraData.BeHitImpact` (`self.ChargeHitImpact`) _returnvalue_2)
                  (`/Game/_Game/AbilitySystem/BP_AbilityFunctionLibrary.ApplyHitDamageTarget` (`self.HitActor`) (`self.HitEventData`) (`self.ChargeBaseDamage`) _returnvalue_2))))))))))

(fn `GetChargeAttackInfoByStickEnergy`
  (returns (SecctionName :type Name) (CostStickEnergy :type "Float (double-precision)") (BaseDamage :type "Float (double-precision)") (HitImpact :type "Float (double-precision)"))
  (locals (StickEnergy :type "Float (single-precision)" :default 0.0))
  (`|ExecutionSequence`
    (:`then_0`
      (set `local.StickEnergy` (`WKHealthComponent.GetStickEnergy` (`WKCharacterBase.HealthComponent` (`self.GetWKCharacterFromActorInfo`)))))
    (:`then_1`
      (if (`KismetMathLibrary.InRange_FloatFloat` (`local.StickEnergy`) 0.0 100.0 true false)
        (return "Charge01" (`local.StickEnergy`) 10.0 100.0)
        (elif (`KismetMathLibrary.InRange_FloatFloat` (`local.StickEnergy`) 100.0 200.0 true false)
          (return "Charge02" (`local.StickEnergy`) 20.0 200.0)
          (elif (`KismetMathLibrary.InRange_FloatFloat` (`local.StickEnergy`) 200.0 300.0 true false)
            (return "Charge03" (`local.StickEnergy`) 30.0 300.0)
            (else
              (return "Charge04" (`local.StickEnergy`) 40.0 300.0))))))))