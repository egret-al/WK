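; Wu Kong's dodge ability, playing a front, back, left or right montage section picked from movement acceleration relative to facing.
; A tick task times the perfect-dodge window and removes the Invincible tag when it expires.
; An attack detection inside the window sends a PerfectDodge event with the direction tag and ends the ability; a later one just ends it.
; A ShouldMove event unblocks movement, letting move input end the dodge early and clear the combo index.
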(event `self.K2_ActivateAbility`
  (bind _returnvalue (`self.GetWKCharacterFromActorInfo`))
  (bind (_sectionname _sectiontag) (`self.GetDodgeInfo`))
  (`self.K2_CommitAbility`)
  (set `self.HasPerfectDodge` false)
  (set `self.PerfectTimeout` false)
  (set `self.CurrentTime` 0.0)
  (set `self.SectionTag` _sectiontag)
  (`WKAbilityTask_PlayMontageAndWaitForEvent.PlayMontageAndWaitForEvent` "None" (`self.DodgeMontage`) (struct) 1.0 _sectionname
    (:`then`
      (`|ExecutionSequence`
        (:`then_0`
          ;[1 1 1] 提前移动结束闪避
          (`AbilityTask_WaitGameplayEvent.WaitGameplayEvent` (struct :`TagName` "Gameplay.Message.ShouldMove") null
            (:`then`
              (`WKAbilityTask_WaitMoveInput.WaitMoveInput` false
                (:`OnMoveInput`
                  (if (`self.CanMove`)
                    (`/Engine/EditorBlueprintResources/StandardMacros.IsValid` _returnvalue
                      (:`Is Valid`
                        (`WKCharacterBase.ClearMeleeComboIndex` _returnvalue)
                        (`self.K2_EndAbility`)))))))
            (:`EventReceived`
              (set `self.CanMove` true)
              (`self.RemoveGameplayTag` (struct :`TagName` "Gameplay.State.Input.BlockMove")))))
        (:`then_1`
          ;[1 1 1] 计时，计算完美闪避窗口期是否过了
          (bind (_asynctaskproxy _deltatime) (`WKAbilityTask_TickTask.TickTask` -1.0)
            (:`then`
              (set `self.AsyncTask_PerfectDodgeWindow` _asynctaskproxy))
            (:`OnTickDelegate`
              (set `self.CurrentTime` (+ _deltatime (`self.CurrentTime`)))
              (if (and (> (`self.CurrentTime`) (`self.PerfectWindow`)) (not (`self.PerfectTimeout`)))
                (set `self.PerfectTimeout` true)
                (`self.RemoveGameplayTag` (struct :`TagName` "Gameplay.State.Invincible"))
                (`GameplayTask.EndTask` (`self.AsyncTask_PerfectDodgeWindow`))))))
        (:`then_2`
          ;[1 1 1] 闪避过程中被敌方攻击检测到，进行完美闪避的判定
          (`AbilityTask_WaitGameplayEvent.WaitGameplayEvent` (struct :`TagName` "Gameplay.Message.Attack.Detection") null
            (:`EventReceived`
              (if (`self.PerfectTimeout`)
                (`self.K2_EndAbility`)
                (elif (not (`self.HasPerfectDodge`))
                  (set `self.HasPerfectDodge` true)
                  (`AbilitySystemBlueprintLibrary.SendGameplayEventToActor` (`self.GetWKCharacterFromActorInfo`) (struct :`TagName` "Gameplay.Event.PerfectDodge") (make `GameplayEventData` (struct) null null null null (struct) (struct) (`BlueprintGameplayTagLibrary.MakeGameplayTagContainerFromTag` (`self.SectionTag`))))
                  (`self.K2_EndAbility`))))))))
    (:`OnCompleted`
      (`self.K2_EndAbility` :!label _label))
    (:`OnBlendOut`
      (goto _label))
    (:`OnInterrupted`
      (goto _label))
    (:`OnCancelled`
      (goto _label))
    (:`OnMontageStop`
      (goto _label))))

(event `self.K2_OnEndAbility`
  (params (bWasCancelled :type Boolean)))

(fn `GetDodgeInfo`
  (returns (SectionName :type Name) (SectionTag :type "GameplayTag Structure"))
  (locals (Angle :type "Float (double-precision)" :default 0.0))
  (bind _returnvalue (`self.GetWKCharacterFromActorInfo`))
  (bind (_returnvalue_x _returnvalue_y) (`KismetMathLibrary.BreakVector` (`KismetMathLibrary.LessLess_VectorRotator` (`CharacterMovementComponent.GetCurrentAcceleration` (`Character.CharacterMovement` _returnvalue)) (`Actor.K2_GetActorRotation` _returnvalue))))
  ;[1 1 1] 根据玩家当前角色的朝向和输入的朝向，来决定使用的是朝着哪个方向的闪避
  (set `local.Angle` (`KismetMathLibrary.DegAtan2` _returnvalue_y _returnvalue_x))
  (if (`KismetMathLibrary.InRange_FloatFloat` (`local.Angle`) -45.0 45.0)
    (return "DodgeF" (struct :`TagName` "Gameplay.EventData.DodgeF"))
    (elif (`KismetMathLibrary.InRange_FloatFloat` (`local.Angle`) -135.0 -45.0)
      (return "DodgeL" (struct :`TagName` "Gameplay.EventData.DodgeL"))
      (elif (`KismetMathLibrary.InRange_FloatFloat` (`local.Angle`) 45.0 135.0)
        (return "DodgeR" (struct :`TagName` "Gameplay.EventData.DodgeR"))
        (else
          (return "DodgeB" (struct :`TagName` "Gameplay.EventData.DodgeB")))))))