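; WuKong's perfect dodge gameplay ability, which plays a directional dodge montage section chosen from the triggering event's target tag.
; It halves global time dilation and spawns an afterimage from the character's skeletal mesh.
; A tick task restores normal time after a set duration, as does ending the ability.
; A ShouldMove event unblocks movement, letting move input end the dodge early and clear the melee combo index.
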(event `self.K2_ActivateAbilityFromEvent`
  (params (EventData :type "GameplayEventData Structure (by ref)"))
  (bind _returnvalue (`self.GetWKCharacterFromActorInfo`))
  (bind _gameplaytags (`BlueprintGameplayTagLibrary.BreakGameplayTagContainer` (`.TargetTags` (break `GameplayEventData` EventData))))
  (bind _returnvalue_2 (`WKCharacterBase.GetWKSkeletalMeshComponent` (`self.GetWKCharacterFromActorInfo`)))
  (bind (_sectionname _success) (`self.GetSectionName` (`|GetArrayItem` _gameplaytags)))
  (`self.K2_CommitAbility`)
  (if (`KismetArrayLibrary.Array_IsEmpty` _gameplaytags)
    (`self.K2_EndAbility`)
    (elif _success
      (`WKAbilityTask_PlayMontageAndWaitForEvent.PlayMontageAndWaitForEvent` "None" (`self.DodgeMontage`) (struct) 1.0 _sectionname
        (:`then`
          (`|ExecutionSequence`
            (:`then_0`
              ;[1 1 1] 完美闪避残影、时间膨胀
              (`GameplayStatics.SetGlobalTimeDilation` 0.5)
              (set `self.PerfectDodgeTimeDilation` 0.0)
              (bind (_asynctaskproxy _deltatime) (`WKAbilityTask_TickTask.TickTask` -1.0)
                (:`then`
                  (set `self.AsyncTask_PerfectDodgeTimeDilationRestore` _asynctaskproxy)
                  (`|SpawnActorFromClass` "/Game/_Game/Character/WuKong/Animation/AnimMontage/Afterimage/BP_DodgeAfterimagePose.BP_DodgeAfterimagePose_C" (`SceneComponent.K2_GetComponentToWorld` _returnvalue_2) "Undefined" "MultiplyWithRoot" null _returnvalue_2 null))
                (:`OnTickDelegate`
                  (bind _output_get (set `self.PerfectDodgeTimeDilation` (+ _deltatime (`self.PerfectDodgeTimeDilation`))))
                  (if (> _output_get (`self.PerfectDodgeRestoreTimeDilation`))
                    (`GameplayTask.EndTask` (`self.AsyncTask_PerfectDodgeTimeDilationRestore`))
                    (`GameplayStatics.SetGlobalTimeDilation` 1.0)))))
            (:`then_1`
              ;[1 1 1] 提前移动结束闪避
              (`AbilityTask_WaitGameplayEvent.WaitGameplayEvent` (struct :`TagName` "Gameplay.Message.ShouldMove") null
                (:`then`
                  (`WKAbilityTask_WaitMoveInput.WaitMoveInput` false
                    (:`OnMoveInput`
                      (if (`self.CanMove`)
                        (`/Engine/EditorBlueprintResources/StandardMacros.IsValid` _returnvalue
                          (:`Is Valid`
                            (`WKCharacterBase.ClearMeleeComboIndex` _returnvalue)
                            (`self.K2_EndAbility`)))))))
                (:`EventReceived`
                  (set `self.CanMove` true)
                  (`self.RemoveGameplayTag` (struct :`TagName` "Gameplay.State.Input.BlockMove")))))))
        (:`OnCompleted`
          (`self.K2_EndAbility` :!label _label))
        (:`OnBlendOut`
          (goto _label))
        (:`OnInterrupted`
          (goto _label))
        (:`OnCancelled`
          (goto _label))
        (:`OnMontageStop`
          (goto _label)))
      (else
        (`self.K2_EndAbility`)))))

(event `self.K2_OnEndAbility`
  (params (bWasCancelled :type Boolean))
  (`GameplayStatics.SetGlobalTimeDilation` 1.0))

(fn `GetSectionName`
  (params (SectionTag :type "GameplayTag Structure"))
  (returns (SectionName :type Name) (Success :type Boolean))
  (if (== SectionTag (struct :`TagName` "Gameplay.EventData.DodgeB"))
    (return "DodgeB" true)
    (elif (== (`local.SectionTag`) (struct :`TagName` "Gameplay.EventData.DodgeF"))
      (return "DodgeF" true)
      (elif (== (`local.SectionTag`) (struct :`TagName` "Gameplay.EventData.DodgeL"))
        (return "DodgeL" true)
        (elif (== (`local.SectionTag`) (struct :`TagName` "Gameplay.EventData.DodgeR"))
          (return "DodgeR" true)
          (else
            (return "None" false)))))))