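; Wukong's Resolute Counterflow ability, a combo counter attack whose follow-up stage unlocks only after the first hits or a counter succeeds.
; Each activation advances the combo index, selecting a montage section, damage and impact, with montage hit events applying damage.
; An incoming attack during invincibility counts as a successful counter with brief global slow motion; otherwise it ends the ability.
; A montage event allows movement input to cancel early and reset the combo.
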(event `self.K2_PreActivate`
  (params (TriggerEventData :type "GameplayEventData Structure (by ref)"))
  (bind _returnvalue (`self.GetWKCharacterFromActorInfo`))
  (`WKCharacterBase.ClearMeleeComboIndex` _returnvalue)
  (`WKCharacterBase.SetCounterComboIndex` _returnvalue (mod (+ (`WKCharacterBase.CurrentCounterComboIndex` _returnvalue) 1) (`self.CounterMaxIndex`)))
  (set `self.IsFirstCounterCombo` (== (`WKCharacterBase.CurrentCounterComboIndex` _returnvalue) 0)))

(event `self.K2_ActivateAbility`
  (bind _returnvalue (`self.GetWKCharacterFromActorInfo`))
  (bind (_montage _name _basedamage _hitimpact) (`self.GetCounterComboMontage`))
  (`CharacterMovementComponent.SetMovementMode` (`Character.CharacterMovement` (`self.GetWKCharacterFromActorInfo`)) "MOVE_Flying" 0)
  (set `self.CanMove` false)
  (set `self.BaseDamage` _basedamage)
  (set `self.HitImpact` _hitimpact)
  (bind (_asynctaskproxy _eventtag _eventdata) (`WKAbilityTask_PlayMontageAndWaitForEvent.PlayMontageAndWaitForEvent` "None" _montage (struct :`GameplayTags` (struct :`(TagName` "Gameplay.Message.Damage.Hit"))) 1.0 _name)
    (:`then`
      (`|ExecutionSequence`
        (:`then_0`
          ;[1 1 1] 检查提前移动
          (`AbilityTask_WaitGameplayEvent.WaitGameplayEvent` (struct :`TagName` "Gameplay.Message.ShouldMove") null
            (:`then`
              (`WKAbilityTask_WaitMoveInput.WaitMoveInput` false
                (:`OnMoveInput`
                  (if (`self.CanMove`)
                    (`/Engine/EditorBlueprintResources/StandardMacros.IsValid` _returnvalue
                      (:`Is Valid`
                        (`WKCharacterBase.ClearCounterComboIndex` _returnvalue)
                        (`self.K2_EndAbility`)))))))
            (:`EventReceived`
              (set `self.CanMove` true)
              (`self.RemoveGameplayTag` (struct :`TagName` "Gameplay.State.Input.BlockMove")))))
        (:`then_1`
          ;[1 1 1] 检查被命中
          (set `self.CounterSuccess` false)
          (`AbilityTask_WaitGameplayEvent.WaitGameplayEvent` (struct :`TagName` "Gameplay.Message.Attack.Detection") null
            (:`EventReceived`
              (if (`WKAbilitySystemComponent.HasMatchingGameplayTagExactly` (`self.GetWKAbilitySystemComponentFromActorInfo`) (struct :`TagName` "Gameplay.State.Invincible"))
                (if (not (`self.CounterSuccess`))
                  ;[1 1 1] 识破成功，做一些表现效果
                  (set `self.CounterSuccess` true)
                  (set `self.CurrentTimeDilationDuration` 0.0)
                  (set `self.ShouldReleaseCounterCombo` true)
                  (`GameplayStatics.SetGlobalTimeDilation` 0.5)
                  (bind (_asynctaskproxy_2 _deltatime) (`WKAbilityTask_TickTask.TickTask` -1.0)
                    (:`then`
                      (set `self.AsyncTask_TimeDilation` _asynctaskproxy_2))
                    (:`OnTickDelegate`
                      (bind _output_get (set `self.CurrentTimeDilationDuration` (+ _deltatime (`self.CurrentTimeDilationDuration`))))
                      (if (>= _output_get (`self.TimeDilationDuration`))
                        (`GameplayStatics.SetGlobalTimeDilation` 1.0)
                        (`GameplayTask.EndTask` (`self.AsyncTask_TimeDilation`))))))
                (else
                  (`self.K2_EndAbility`))))))))
    (:`OnCompleted`
      (`self.K2_EndAbility` :!label _label))
    (:`OnBlendOut`
      (goto _label))
    (:`OnInterrupted`
      (goto _label))
    (:`OnCancelled`
      (goto _label))
    (:`EventReceived`
      (if (== _eventtag (struct :`TagName` "Gameplay.Message.Damage.Hit"))
        (bind _output_get_2 (set `self.HitEventData` _eventdata))
        (bind _aswkcharacter_base (cast `WKCharacterBase` (`.Target` (break `GameplayEventData` _output_get_2))))
        (bind _output_get_3 (set `self.HitActor` _aswkcharacter_base))
        (bind _output_get_4 (set `self.HitActorASC` (`WKGameplayStatics.GetWKAbilitySystemComponent` _output_get_3)))
        (`/Engine/EditorBlueprintResources/StandardMacros.IsValid` _output_get_4
          (:`Is Valid`
            (`|ExecutionSequence`
              (:`then_0`
                ;[1 1 1] 命中到目标了
                (`self.CheckAndSetNextCounterCombo`)
                (bind _returnvalue_2 (`|GenericCreateObject` "/Script/BlackWK.WKCharacterBeHitEventExtraData"))
                (set `WKCharacterBeHitEventExtraData.Instigator` (`self.GetWKCharacterFromActorInfo`) _returnvalue_2)
                (set `WKCharacterBeHitEventExtraData.AbilityDataAsset` (`self.AbilityDataAsset`) _returnvalue_2)
                (set `WKCharacterBeHitEventExtraData.BeHitImpact` (`self.HitImpact`) _returnvalue_2)
                (`/Game/_Game/AbilitySystem/BP_AbilityFunctionLibrary.ApplyHitDamageTarget` (`self.HitActor`) (`self.HitEventData`) (`self.BaseDamage`) _returnvalue_2)))))))))

(event `self.K2_OnEndAbility`
  (params (bWasCancelled :type Boolean))
  (`CharacterMovementComponent.SetMovementMode` (`Character.CharacterMovement` (`self.GetWKCharacterFromActorInfo`)) "MOVE_Walking" 0)
  (`GameplayStatics.SetGlobalTimeDilation` 1.0)
  ;[1 1 1] 第二段结束后，应该重置第二段开启条件
  (if (not (`self.IsFirstCounterCombo`))
    (set `self.ShouldReleaseCounterCombo` false)))

(fn `CheckAndSetNextCounterCombo`
  ;[1 1 1] 只有第一段Counter才能去修改第二段的
  (if (`self.IsFirstCounterCombo`)
    (set `self.ShouldReleaseCounterCombo` true)))

(fn `GetCounterComboMontage`
  (returns (Montage :type "AnimMontage Object Reference") (Name :type Name) (BaseDamage :type "Float (double-precision)") (HitImpact :type "Float (double-precision)"))
  (bind _currentcountercomboindex (`WKCharacterBase.CurrentCounterComboIndex` (`self.GetWKCharacterFromActorInfo`)))
  (return "/Game/_Game/Character/WuKong/Animation/AnimMontage/AM_ResoluteCounterflow_Combo.AM_ResoluteCounterflow_Combo" (`|GetArrayItem` (`self.CounterComboNames`) _currentcountercomboindex) (`|GetArrayItem` (`self.BaseDamages`) _currentcountercomboindex) (`|GetArrayItem` (`self.CounterHitImpacts`) _currentcountercomboindex)))

(fn `K2_CanActivateAbility`
  (params (ActorInfo :type "GameplayAbilityActorInfo Structure") (Handle :type "GameplayAbilitySpecHandle Structure"))
  (returns (RelevantTags :type "GameplayTagContainer Structure") (ReturnValue :type Boolean))
  (locals (LocalCurrentCounterComboIndex :type Integer :default 0))
  ;[1 1 1] 第一段Counter直接放，但是第二段就需要检查第一段是否有命中人或者说是否有识破成功
  (bind _output_get (set `local.LocalCurrentCounterComboIndex` (`WKCharacterBase.CurrentCounterComboIndex` (`self.GetWKCharacterFromActorInfo`))))
  (if (< _output_get 0)
    (return (struct) true)
    (else
      (return (struct) (`self.ShouldReleaseCounterCombo`)))))