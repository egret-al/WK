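; Gameplay ability that roots the WuKong character by freezing it for a set duration.
; On event activation it sets the character's CustomTimeDilation to zero, halting its own time rather than only blocking movement, and clears the melee combo index.
; A DelayTask ends the ability after RootedTime, and OnEndAbility restores normal time dilation.
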(event `self.K2_ActivateAbilityFromEvent`
  (params (EventData :type "GameplayEventData Structure (by ref)"))
  (bind _returnvalue (`self.GetWKCharacterFromActorInfo`))
  (`/Engine/EditorBlueprintResources/StandardMacros.IsValid` _returnvalue
    (:`Is Valid`
      (set `Actor.CustomTimeDilation` 0.0 _returnvalue)
      (`WKCharacterBase.ClearMeleeComboIndex` _returnvalue)
      (`WKAbilityTask_DelayTask.DelayTask` (`self.RootedTime`)
        (:`OnDelayDelegate`
          (`self.K2_EndAbility`))))
    (:`Is Not Valid`
      (`self.K2_EndAbility`))))

(event `self.K2_OnEndAbility`
  (params (bWasCancelled :type Boolean))
  (bind _returnvalue (`self.GetWKCharacterFromActorInfo`))
  (`/Engine/EditorBlueprintResources/StandardMacros.IsValid` _returnvalue
    (:`Is Valid`
      (set `Actor.CustomTimeDilation` 1.0 _returnvalue))))