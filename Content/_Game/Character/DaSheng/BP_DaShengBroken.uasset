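; BP_DaShengBroken is a Da Sheng character Blueprint with an enemy health bar, hit reactions and a lock point.
; On BeginPlay it casts its widget component's widget to WBP_EnemyHealthBar and initializes it with itself.
; PlayHitMontage plays the Da Sheng hit montage from a randomly picked section for varied reactions.
; GetLockLocation returns the mesh's LockSocket position.
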(event `self.ReceiveBeginPlay`
  (bind _aswbp_enemy_health_bar (cast `/Game/_Game/UI/HUD/WBP_EnemyHealthBar` (`WidgetComponent.GetWidget` (`self.Widget`))))
  (`/Game/_Game/UI/HUD/WBP_EnemyHealthBar.InitializeWidget` _aswbp_enemy_health_bar self))

(event `self.PlayHitMontage`
  (params (InInstigator :type "WKCharacterBase Object Reference"))
  (`|PlayMontage` (`self.Mesh`) "/Game/_Game/Character/DaSheng/Animation/AnimMontage/AM_Hit_DaSheng.AM_Hit_DaSheng" 1.0 0.0 (`KismetArrayLibrary.Array_Random` (`self.HitSectionNames`))))

(fn `GetLockLocation`
  (returns (ReturnValue :type "Vector Structure"))
  (return (`SceneComponent.GetSocketLocation` (`self.Mesh`) "LockSocket")))

(fn `UserConstructionScript`)