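; BP_WuKong is the WuKong character Blueprint, currently acting mostly as a movement debugging view.
; Tick draws debug arrows from the actor for current acceleration (red) and scaled facing direction (green).
; SmoothCharacterRotation chases a target rotation with constant-speed interpolation, then eases the actor toward it for two-stage smoothing.
; Its only caller, driven by the animation instance's RotationAmount curve, is disconnected and never runs.
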(event `self.ReceiveBeginPlay`)

(event `self.ReceiveTick`
  (params (DeltaSeconds :type "Float (single-precision)"))
  (bind _returnvalue (`self.K2_GetActorLocation`))
  (bind _returnvalue_2 (`self.K2_GetActorLocation`))
  (`KismetSystemLibrary.DrawDebugArrow` _returnvalue_2 (+ _returnvalue_2 (`CharacterMovementComponent.GetCurrentAcceleration` (`self.CharacterMovement`))) 1.0 (struct :`R` 1.0 :`G` 0.137657 :`A` 1.0) 0.0 1.0)
  (`KismetSystemLibrary.DrawDebugArrow` _returnvalue (+ _returnvalue (* (`self.GetActorForwardVector`) (`self.NewVar`))) 1.0 (struct :`R` 0.144386 :`G` 1.0 :`A` 1.0) 0.0 1.0))

(fn `SmoothCharacterRotation`
  (params (Target :type "Rotator Structure") (`TargetInterpSpeed(Const)` :type "Float (double-precision)") (`ActorInterpSpeed(Smooth)` :type "Float (double-precision)"))
  (set `self.TargetRotation` (`KismetMathLibrary.RInterpTo_Constant` (`self.TargetRotation`) (`local.Target`) (`GameplayStatics.GetWorldDeltaSeconds`) (`local.TargetInterpSpeed(Const)`)))
  (`self.K2_SetActorRotation` (`KismetMathLibrary.RInterpTo` (`self.K2_GetActorRotation`) (`self.TargetRotation`) (`GameplayStatics.GetWorldDeltaSeconds`) (`local.ActorInterpSpeed(Smooth)`))))

(fn `UserConstructionScript`)